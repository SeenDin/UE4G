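; BP_Character is a player character with axis-driven walking and look controls and a toggleable camera.
; Movement input follows the capsule's right and forward vectors, while look axes feed controller pitch and yaw.
; The forward/back axis also sets max walk speed each update, halving it when the input is fully backward.
; The ChangeCamera action uses a FlipFlop to swap the active camera between Camera1 and Camera3.
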(event `InputAxis|MoveLeftRight`
  (params (AxisValue :type "Float (single-precision)"))
  (`self.AddMovementInput` (`SceneComponent.GetRightVector` (`self.CapsuleComponent`)) AxisValue))

(event `InputAxis|MoveForwardBack`
  (params (AxisValue :type "Float (single-precision)"))
  (bind _charactermovement (`self.CharacterMovement`))
  (`self.AddMovementInput` (`SceneComponent.GetForwardVector` (`self.CapsuleComponent`)) AxisValue)
  (set `CharacterMovementComponent.MaxWalkSpeed` 300.0 _charactermovement)
  (if (== AxisValue -1.0)
    (set `CharacterMovementComponent.MaxWalkSpeed` 150.0 _charactermovement)))

(event `InputAxis|LookUpDown`
  (params (AxisValue :type "Float (single-precision)"))
  (`self.AddControllerPitchInput` AxisValue))

(event `InputAxis|LookLeftRight`
  (params (AxisValue :type "Float (single-precision)"))
  (`self.AddControllerYawInput` AxisValue))

(event `InputAction|ChangeCamera`
  (params (Key :type "Key Structure"))
  (:`Pressed`
    (`/Engine/EditorBlueprintResources/StandardMacros.FlipFlop`
      (:`A`
        (`ActorComponent.Deactivate` (`self.Camera3`))
        (`ActorComponent.Activate` (`self.Camera1`) false))
      (:`B`
        (`ActorComponent.Deactivate` (`self.Camera1`))
        (`ActorComponent.Activate` (`self.Camera3`) false)))))

(fn `UserConstructionScript`)